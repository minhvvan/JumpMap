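; BP_AnimActor is an animated actor that slides along its arrow's direction while its Heart component spins.
; On BeginPlay it stores its start location and plays the 이동그래프 (movement graph) timeline, whose track scales an offset along the Arrow's forward vector from that point.
; Tick adds a fixed rotation to Heart every frame, so the spin speed depends on frame rate.
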(event EventBeginPlay
  (Variables|Default|SetInitPos (Transformation|GetActorLocation))
  (bind _새_트랙_0 (Timeline|이동그래프 Play)
    (:Update
      (Transformation|SetActorLocation (+ (Variables|Default|GetInitPos) (* (Math|Vector|GetForwardVector (Variables|Default|GetArrow)) (* _새_트랙_0 5e+01))) false false))))

(event Collision|EventActorBeginOverlap
  (params (OtherActor :type Actor%20Object%20Reference)))

(event EventTick
  (params (DeltaSeconds :type Float%20%28single-precision%29))
  (Transformation|SetWorldRotation (Variables|Default|GetHeart) (Math|Rotator|CombineRotators (Transformation|GetWorldRotation (Variables|Default|GetHeart)) "0.000000,1.000000,0.000000") false false))

(fn ConstructionScript)